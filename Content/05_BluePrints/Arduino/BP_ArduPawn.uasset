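; Player pawn that drives a staged narrative game from physical chips read by an Arduino over a serial port.
; Number keys pick the COM port, and Tick reads lines into a StateValue state machine that accepts the expected chip and fires the matching Movimiento dispatcher.
; Other states handle noise-triggered game over and a Camahueto horn choice, while confirmation starts narration and a ten-minute fail timer.
; Keyboard shortcuts also trigger moves, choices, restart and game over.
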(event Custom|Open%20port
  (params (Port :type Integer))
  ;[1 1 1] Open port
  (Class|SerialCom|Close (Variables|Default|GetMyPort))
  (bind _returnvalue (Class|SerialCom|OpenComPortwithFlowControl Port 9600 true true))
  (if (Class|SerialCom|IsOpened _returnvalue)
    (Variables|Default|SetMyPort _returnvalue)
    (Class|SerialCom|Flush _returnvalue)
    (Variables|Default|SetPortOpen true)))

(event Custom|Wait%2010%20minutes
  (Utilities|FlowControl|Delay 6e+02)
  (CallFunction|GameOver))

(event Custom|Move4
  ;[1 1 1] Eventos Movimiento
  (Default|CallMovimiento4))

(event Custom|Move5
  ;[1 1 1] Eventos Movimiento
  (Default|CallMovimiento5))

(event Custom|GameOver
  (Variables|Default|SetStateValue "vacio")
  (Viewport|RemoveAllWidgets)
  (bind _returnvalue (UserInterface|CreateWidget "/Game/08_UI/PNG/Widget_GameOver.Widget_GameOver_C"))
  (UserInterface|Viewport|AddtoViewport _returnvalue 0))

(event Custom|Move1
  ;[1 1 1] Eventos Movimiento
  (Default|CallMovimiento1))

(event Custom|ConfirmacionInicial
  ;[1 1 1] Confirma
  (Audio|PlaySound2D "/Game/06_Metasound/Tracks/Timeline/Narracion/narrador_1_5.narrador_1_5" 1.0 1.0 0.0 0 0)
  (Utilities|FlowControl|Delay 13.0)
  (Variables|Default|SetStateValue "mov1")
  (CallFunction|Wait10Minutes))

(event Custom|Move6
  ;[1 1 1] Eventos Movimiento
  (Default|CallMovimiento6))

(event Custom|Move2
  ;[1 1 1] Eventos Movimiento
  (Default|CallMovimiento2))

(event Custom|Move3
  ;[1 1 1] Eventos Movimiento
  (Default|CallMovimiento3))

(event EventEndPlay
  (params (EndPlayReason :type EEndPlayReason%20Enum :default "Destroyed"))
  ;[1 1 1] CLose port
  (Class|SerialCom|Close (Variables|Default|GetMyPort)))

(event EventTick
  (params (DeltaSeconds :type Float%20%28single-precision%29))
  ;[1 1 1] Lee el arduino
  (if (Variables|Default|GetPortOpen)
    (bind _returnvalue (Class|SerialCom|Readln (Variables|Default|GetMyPort)))
    (Variables|Default|SetArdValue _returnvalue)
    (if (Utilities|Enum|Equal(Enum) (Variables|Default|GetArdValue) "")
      (Variables|Default|SetChipState false)
      (Variables|Default|SetLastLastRock (Variables|Default|GetLastRock))
      (Variables|Default|SetLastRock (Variables|Default|GetCurrentRock))
      (Variables|Default|SetCurrentRock "")
      (else
        (switch string (Variables|Default|GetStateValue)
          (:inicio
            ;[1 1 1] Confirmacion inicial
            (if (not (Variables|Default|GetChipState))
              (Variables|Default|SetCurrentRock (Variables|Default|GetArdValue))
              (Variables|Default|SetChipState true)
              (CallFunction|ConfirmacionInicial)
              (Variables|Default|SetStateValue "vacio")))
          (:mov1
            ;[1 1 1] Movimiento1
            (if (not (Variables|Default|GetChipState))
              (Variables|Default|SetCurrentRock (Variables|Default|GetArdValue))
              (Variables|Default|SetChipState true)
              (if (Utilities|Enum|Equal(Enum) (Variables|Default|GetArdValue) "chip1")
                (CallFunction|Move1)
                (Variables|Default|SetStateValue "vacio"))))
          (:mov2
            ;[1 1 1] Movimiento2
            (if (not (Variables|Default|GetChipState))
              (Variables|Default|SetCurrentRock (Variables|Default|GetArdValue))
              (Variables|Default|SetChipState true)
              (if (Utilities|Enum|Equal(Enum) (Variables|Default|GetArdValue) "chip2")
                (CallFunction|Move2)
                (Variables|Default|SetStateValue "vacio"))))
          (:ruido
            ;[1 1 1] Evento ruido
            (if (Utilities|Enum|Equal(Enum) (Variables|Default|GetArdValue) "ruido")
              (CallFunction|GameOver)
              (Variables|Default|SetStateValue "vacio")))
          (:mov3
            ;[1 1 1] Movimiento3
            (if (not (Variables|Default|GetChipState))
              (Variables|Default|SetCurrentRock (Variables|Default|GetArdValue))
              (Variables|Default|SetChipState true)
              (if (Utilities|Enum|Equal(Enum) (Variables|Default|GetArdValue) "chip3")
                (CallFunction|Move3)
                (Variables|Default|SetStateValue "vacio"))))
          (:mov4
            ;[1 1 1] Movimiento4
            (if (not (Variables|Default|GetChipState))
              (Variables|Default|SetCurrentRock (Variables|Default|GetArdValue))
              (Variables|Default|SetChipState true)
              (if (Utilities|Enum|Equal(Enum) (Variables|Default|GetArdValue) "chip4")
                (CallFunction|Move4)
                (Variables|Default|SetStateValue "vacio"))))
          (:mov5
            ;[1 1 1] Movimiento5
            (if (not (Variables|Default|GetChipState))
              (Variables|Default|SetCurrentRock (Variables|Default|GetArdValue))
              (Variables|Default|SetChipState true)
              (if (Utilities|Enum|Equal(Enum) (Variables|Default|GetArdValue) "chip1")
                (CallFunction|Move5)
                (Variables|Default|SetStateValue "vacio"))))
          (:mov6
            ;[1 1 1] Movimiento6
            (if (not (Variables|Default|GetChipState))
              (Variables|Default|SetCurrentRock (Variables|Default|GetArdValue))
              (Variables|Default|SetChipState true)
              (if (Utilities|Enum|Equal(Enum) (Variables|Default|GetArdValue) "chip2")
                (CallFunction|Move6)
                (Variables|Default|SetStateValue "vacio"))))
          (:eleccion
            ;[1 1 1] Evento eleccion
            (if (not (Variables|Default|GetChipState))
              (if (Utilities|Enum|Equal(Enum) (Variables|Default|GetArdValue) "chip1")
                (Audio|PlaySound2D "/Game/06_Metasound/Tracks/Camahueto/CamahuetoScream1.CamahuetoScream1" 1.0 1.0 0.0 0 0)
                (Utilities|FlowControl|Delay 2.8)
                (Variables|Default|SetConCuerno true)
                (Variables|Default|SetStateValue "mov6")
                (Viewport|RemoveAllWidgets :!label _label)
                (bind _returnvalue_2 (UserInterface|CreateWidget "/Game/08_UI/PNG/Widget_Codigos.Widget_Codigos_C"))
                (UserInterface|Viewport|AddtoViewport _returnvalue_2 0)
                (elif (Utilities|Enum|Equal(Enum) (Variables|Default|GetArdValue) "chip4")
                  (Audio|PlaySound2D "/Game/06_Metasound/Tracks/Camahueto/CamahuetoScream2.CamahuetoScream2" 1.0 1.0 0.0 0 0)
                  (Utilities|FlowControl|Delay 4.7)
                  (Variables|Default|SetConCuerno false)
                  (Variables|Default|SetStateValue "mov6")
                  (goto _label))))))))))

(event Input|KeyboardEvents|1
  (params (Key :type Key%20Structure :default "None"))
  ;[1 1 1] Keys to open ports
  (:Pressed
    (CallFunction|OpenPort 1)))

(event Input|KeyboardEvents|2
  (params (Key :type Key%20Structure :default "None"))
  ;[1 1 1] Keys to open ports
  (:Pressed
    (CallFunction|OpenPort 2)))

(event Input|KeyboardEvents|Q
  (params (Key :type Key%20Structure :default "None"))
  ;[1 1 1] Keys to open ports
  (:Pressed
    (CallFunction|GameOver)))

(event Input|KeyboardEvents|O
  (params (Key :type Key%20Structure :default "None"))
  (:Pressed
    ;[1 1 1] Evento eleccion
    (Audio|PlaySound2D "/Game/06_Metasound/Tracks/Camahueto/CamahuetoScream2.CamahuetoScream2" 1.0 1.0 0.0 0 0)
    (Utilities|FlowControl|Delay 4.7)
    (Variables|Default|SetConCuerno false)
    (Variables|Default|SetStateValue "mov6")
    (Viewport|RemoveAllWidgets)
    (bind _returnvalue (UserInterface|CreateWidget "/Game/08_UI/PNG/Widget_Codigos.Widget_Codigos_C"))
    (UserInterface|Viewport|AddtoViewport _returnvalue 0)))

(event Input|KeyboardEvents|C
  (params (Key :type Key%20Structure :default "None"))
  (:Pressed
    (CallFunction|Move1)))

(event Input|KeyboardEvents|V
  (params (Key :type Key%20Structure :default "None"))
  (:Pressed
    (CallFunction|Move2)))

(event Input|KeyboardEvents|B
  (params (Key :type Key%20Structure :default "None"))
  (:Pressed
    (CallFunction|Move3)))

(event Input|KeyboardEvents|N
  (params (Key :type Key%20Structure :default "None"))
  (:Pressed
    (CallFunction|Move4)))

(event Input|KeyboardEvents|M
  (params (Key :type Key%20Structure :default "None"))
  (:Pressed
    (CallFunction|Move5)))

(event Input|KeyboardEvents|K
  (params (Key :type Key%20Structure :default "None"))
  (:Pressed
    (CallFunction|Move6)))

(event Input|KeyboardEvents|I
  (params (Key :type Key%20Structure :default "None"))
  (:Pressed
    ;[1 1 1] Evento eleccion
    (Audio|PlaySound2D "/Game/06_Metasound/Tracks/Camahueto/CamahuetoScream1.CamahuetoScream1" 1.0 1.0 0.0 0 0)
    (Utilities|FlowControl|Delay 2.8)
    (Variables|Default|SetConCuerno true)
    (Variables|Default|SetStateValue "mov6")
    (Viewport|RemoveAllWidgets)
    (bind _returnvalue (UserInterface|CreateWidget "/Game/08_UI/PNG/Widget_Codigos.Widget_Codigos_C"))
    (UserInterface|Viewport|AddtoViewport _returnvalue 0)))

(event Input|KeyboardEvents|3
  (params (Key :type Key%20Structure :default "None"))
  ;[1 1 1] Keys to open ports
  (:Pressed
    (CallFunction|OpenPort 3)))

(event Input|KeyboardEvents|4
  (params (Key :type Key%20Structure :default "None"))
  ;[1 1 1] Keys to open ports
  (:Pressed
    (CallFunction|OpenPort 4)))

(event Input|KeyboardEvents|5
  (params (Key :type Key%20Structure :default "None"))
  ;[1 1 1] Keys to open ports
  (:Pressed
    (CallFunction|OpenPort 5)))

(event Input|KeyboardEvents|6
  (params (Key :type Key%20Structure :default "None"))
  ;[1 1 1] Keys to open ports
  (:Pressed
    (CallFunction|OpenPort 6)))

(event Input|KeyboardEvents|7
  (params (Key :type Key%20Structure :default "None"))
  ;[1 1 1] Keys to open ports
  (:Pressed
    (CallFunction|OpenPort 7)))

(event Input|KeyboardEvents|8
  (params (Key :type Key%20Structure :default "None"))
  ;[1 1 1] Keys to open ports
  (:Pressed
    (CallFunction|OpenPort 8)))

(event Input|KeyboardEvents|9
  (params (Key :type Key%20Structure :default "None"))
  ;[1 1 1] Keys to open ports
  (:Pressed
    (CallFunction|OpenPort 9)))

(event Input|KeyboardEvents|R
  (params (Key :type Key%20Structure :default "None"))
  ;[1 1 1] Reset level
  (:Pressed
    (bind _returnvalue (Game|GetCurrentLevelName true))
    (Game|OpenLevel(byName) (Utilities|String|StringToName _returnvalue))))

(fn ConstructionScript)