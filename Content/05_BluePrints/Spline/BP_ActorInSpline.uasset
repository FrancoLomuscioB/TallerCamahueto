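; Actor that drives the game's scripted story sequence by travelling along six spline paths, one per movement event from BP_ArduPawn.
; Each segment's Timeline, rate-scaled by its duration, sets the actor's transform by distance along that spline.
; When a segment finishes, timed sounds and narration play, then the first five update the pawn's StateValue.
; The last picks ending narration by ConCuerno, then calls GameOver.
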(event Custom|Mov6
  (bind _spline6 (Variables|Default|GetSpline6))
  (bind _spline (Variables|/Game/05_BluePrints/Spline/BP_SplinePath5.BP_SplinePath5_C|GetSpline _spline6))
  ;[1 1 1] Ultimo movimiento
  (Components|Timeline|SetPlayRate (Variables|Default|GetT_Mov6) (/ 1.0 (Variables|Default|GetDuration6)))
  (bind _track (Timeline|T_Mov6 PlayFromStart)
    (:Update
      (Transformation|SetActorTransform (Math|Transform|MakeTransform (Spline|GetLocationatDistanceAlongSpline _spline (Math|Float|Lerp 0.0 (Spline|GetSplineLength _spline) _track) "Local") (Spline|GetRotationatDistanceAlongSpline _spline (Math|Float|Lerp 0.0 (Spline|GetSplineLength _spline) _track) "Local") "1.000000,1.000000,1.000000")))
    (:Finished
      (if (Variables|/Game/05_BluePrints/Arduino/BP_ArduPawn.BP_ArduPawn_C|GetConCuerno (Variables|Default|GetAs%20BP%20Ardu%20Pawn))
        (Audio|PlaySound2D "/Game/06_Metasound/Tracks/Timeline/Narracion/narrador_7.narrador_7" 1.0 1.0 0.0 0 0) ; sonido del final
        (Utilities|FlowControl|Delay 8.4)
        (Default|GameOver (Variables|Default|GetAs%20BP%20Ardu%20Pawn))
        (else
          (Audio|PlaySound2D "/Game/06_Metasound/Tracks/Timeline/Narracion/narrador_8.narrador_8" 1.0 1.0 0.0 0 0) ; sonido del final
          (Utilities|FlowControl|Delay 7.5)
          (Default|GameOver (Variables|Default|GetAs%20BP%20Ardu%20Pawn)))))))

(event Custom|Move
  (bind _splineref (Variables|Default|GetSplineRef))
  (bind _spline (Variables|/Game/05_BluePrints/Spline/BP_SplinePath.BP_SplinePath_C|GetSpline _splineref))
  ;[1 1 1] Primer movimiento
  (Components|Timeline|SetPlayRate (Variables|Default|GetT_MoveActor) (/ 1.0 (Variables|Default|GetDuration)))
  (bind _track (Timeline|T_MoveActor PlayFromStart)
    (:Update
      (Transformation|SetActorTransform (Math|Transform|MakeTransform (Spline|GetLocationatDistanceAlongSpline _spline (Math|Float|Lerp 0.0 (Spline|GetSplineLength (Variables|/Game/05_BluePrints/Spline/BP_SplinePath.BP_SplinePath_C|GetSpline (Variables|Default|GetSplineRef))) _track) "Local") (Spline|GetRotationatDistanceAlongSpline _spline (Math|Float|Lerp 0.0 (Spline|GetSplineLength (Variables|/Game/05_BluePrints/Spline/BP_SplinePath.BP_SplinePath_C|GetSpline (Variables|Default|GetSplineRef))) _track) "Local") "1.000000,1.000000,1.000000")))
    (:Finished
      (Audio|PlaySound2D "/Game/06_Metasound/Tracks/Timeline/EnfermedadMaxima.EnfermedadMaxima" 1.0 1.0 0.0 0 0) ; persona enferma
      (Utilities|FlowControl|Delay 6.0)
      (Variables|/Game/05_BluePrints/Arduino/BP_ArduPawn.BP_ArduPawn_C|SetStateValue (Variables|Default|GetAs%20BP%20Ardu%20Pawn) "mov2"))))

(event Custom|Move2
  (bind _spline2 (Variables|Default|GetSpline2))
  (bind _spline (Variables|/Game/05_BluePrints/Spline/BP_SplinePath1.BP_SplinePath1_C|GetSpline _spline2))
  ;[1 1 1] Segundo movimiento
  (Components|Timeline|SetPlayRate (Variables|Default|GetT_Move2) (/ 1.0 (Variables|Default|GetDuration2)))
  (bind _track (Timeline|T_Move2 PlayFromStart)
    (:Update
      (Transformation|SetActorTransform (Math|Transform|MakeTransform (Spline|GetLocationatDistanceAlongSpline _spline (Math|Float|Lerp 0.0 (Spline|GetSplineLength (Variables|/Game/05_BluePrints/Spline/BP_SplinePath1.BP_SplinePath1_C|GetSpline (Variables|Default|GetSpline2))) _track) "Local") (Spline|GetRotationatDistanceAlongSpline _spline (Math|Float|Lerp 0.0 (Spline|GetSplineLength (Variables|/Game/05_BluePrints/Spline/BP_SplinePath1.BP_SplinePath1_C|GetSpline (Variables|Default|GetSpline2))) _track) "Local") "1.000000,1.000000,1.000000")))
    (:Finished
      (Audio|PlaySound2D "/Game/06_Metasound/Tracks/Timeline/Cura.Cura" 1.0 1.0 0.0 0 0) ; brujo curando
      (Utilities|FlowControl|Delay 3.5)
      (Audio|PlaySound2D "/Game/06_Metasound/Tracks/Timeline/Narracion/narrador_4.narrador_4" 1.0 1.0 0.0 0 0) ; brujo habla del cuerno
      (Utilities|FlowControl|Delay 3.8)
      (Variables|/Game/05_BluePrints/Arduino/BP_ArduPawn.BP_ArduPawn_C|SetStateValue (Variables|Default|GetAs%20BP%20Ardu%20Pawn) "mov3"))))

(event Custom|Mov3
  (bind _spline3 (Variables|Default|GetSpline3))
  (bind _spline (Variables|/Game/05_BluePrints/Spline/BP_SplinePath2.BP_SplinePath2_C|GetSpline _spline3))
  ;[1 1 1] Tercer movimiento
  (Components|Timeline|SetPlayRate (Variables|Default|GetT_Mov3) (/ 1.0 (Variables|Default|GetDuration3)))
  (bind _track (Timeline|T_Mov3 PlayFromStart)
    (:Update
      (Transformation|SetActorTransform (Math|Transform|MakeTransform (Spline|GetLocationatDistanceAlongSpline _spline (Math|Float|Lerp 0.0 (Spline|GetSplineLength (Variables|/Game/05_BluePrints/Spline/BP_SplinePath2.BP_SplinePath2_C|GetSpline (Variables|Default|GetSpline3))) _track) "Local") (Spline|GetRotationatDistanceAlongSpline _spline (Math|Float|Lerp 0.0 (Spline|GetSplineLength (Variables|/Game/05_BluePrints/Spline/BP_SplinePath2.BP_SplinePath2_C|GetSpline (Variables|Default|GetSpline3))) _track) "Local") "1.000000,1.000000,1.000000")))
    (:Finished
      (Audio|PlaySound2D "/Game/06_Metasound/Tracks/Timeline/Terremoto.Terremoto" 1.0 1.0 0.0 0 0) ; terremoto
      (Utilities|FlowControl|Delay 1e+01)
      (Audio|PlaySound2D "/Game/06_Metasound/Tracks/Timeline/Narracion/narrador_3.narrador_3" 1.0 1.0 0.0 0 0) ; terremoto
      (Utilities|FlowControl|Delay 3.8)
      (Audio|PlaySound2D "/Game/06_Metasound/Tracks/Timeline/Narracion/narrador_5.narrador_5" 1.0 1.0 0.0 0 0) ; terremoto
      (Utilities|FlowControl|Delay 4.0)
      (Variables|/Game/05_BluePrints/Arduino/BP_ArduPawn.BP_ArduPawn_C|SetStateValue (Variables|Default|GetAs%20BP%20Ardu%20Pawn) "mov4"))))

(event Custom|Mov4
  (bind _spline4 (Variables|Default|GetSpline4))
  (bind _spline (Variables|/Game/05_BluePrints/Spline/BP_SplinePath3.BP_SplinePath3_C|GetSpline _spline4))
  ;[1 1 1] Cuarto movimiento
  (Components|Timeline|SetPlayRate (Variables|Default|GetT_Mov4) (/ 1.0 (Variables|Default|GetDuration4)))
  (bind _track (Timeline|T_Mov4 PlayFromStart)
    (:Update
      (Transformation|SetActorTransform (Math|Transform|MakeTransform (Spline|GetLocationatDistanceAlongSpline _spline (Math|Float|Lerp 0.0 (Spline|GetSplineLength _spline) _track) "Local") (Spline|GetRotationatDistanceAlongSpline _spline (Math|Float|Lerp 0.0 (Spline|GetSplineLength _spline) _track) "Local") "1.000000,1.000000,1.000000")))
    (:Finished
      (Audio|PlaySound2D "/Game/06_Metasound/Tracks/Camahueto/CamahuetoScream3.CamahuetoScream3" 1.0 1.0 0.0 0 0) ; ataque del camahueto
      (Utilities|FlowControl|Delay 5.0)
      (Variables|/Game/05_BluePrints/Arduino/BP_ArduPawn.BP_ArduPawn_C|SetStateValue (Variables|Default|GetAs%20BP%20Ardu%20Pawn) "ruido")
      (Audio|PlaySound2D "/Game/06_Metasound/MTSource/CamahuetoTest.CamahuetoTest" 1.0 1.0 0.0 0 0) ; ataque del camahueto
      (Utilities|FlowControl|Delay 2.0)
      (Audio|PlaySound2D "/Game/06_Metasound/MTSource/CamahuetoTest.CamahuetoTest" 1.0 1.0 0.0 0 0) ; ataque del camahueto
      (Utilities|FlowControl|Delay 2.0)
      (Audio|PlaySound2D "/Game/06_Metasound/MTSource/CamahuetoTest.CamahuetoTest" 1.0 1.0 0.0 0 0) ; ataque del camahueto
      (Utilities|FlowControl|Delay 2.0)
      (Audio|PlaySound2D "/Game/06_Metasound/MTSource/CamahuetoTest.CamahuetoTest" 1.0 1.0 0.0 0 0) ; ataque del camahueto
      (Utilities|FlowControl|Delay 2.0)
      (Audio|PlaySound2D "/Game/06_Metasound/MTSource/CamahuetoTest.CamahuetoTest" 1.0 1.0 0.0 0 0) ; ataque del camahueto
      (Utilities|FlowControl|Delay 2.0)
      (Variables|/Game/05_BluePrints/Arduino/BP_ArduPawn.BP_ArduPawn_C|SetStateValue (Variables|Default|GetAs%20BP%20Ardu%20Pawn) "mov5"))))

(event Custom|Mov5
  (bind _spline5 (Variables|Default|GetSpline5))
  (bind _spline (Variables|/Game/05_BluePrints/Spline/BP_SplinePath4.BP_SplinePath4_C|GetSpline _spline5))
  ;[1 1 1] Quinto movimiento
  (Components|Timeline|SetPlayRate (Variables|Default|GetT_Mov5) (/ 1.0 (Variables|Default|GetDuration5)))
  (bind _track (Timeline|T_Mov5 PlayFromStart)
    (:Update
      (Transformation|SetActorTransform (Math|Transform|MakeTransform (Spline|GetLocationatDistanceAlongSpline _spline (Math|Float|Lerp 0.0 (Spline|GetSplineLength _spline) _track) "Local") (Spline|GetRotationatDistanceAlongSpline _spline (Math|Float|Lerp 0.0 (Spline|GetSplineLength _spline) _track) "Local") "1.000000,1.000000,1.000000")))
    (:Finished
      (Audio|PlaySound2D "/Game/06_Metasound/Tracks/Timeline/Narracion/narrador_6.narrador_6" 1.0 1.0 0.0 0 0)
      (Utilities|FlowControl|Delay 7.0)
      (Variables|/Game/05_BluePrints/Arduino/BP_ArduPawn.BP_ArduPawn_C|SetStateValue (Variables|Default|GetAs%20BP%20Ardu%20Pawn) "eleccion"))))

(event EventBeginPlay
  (Utilities|FlowControl|Sequence
    (:then_0
      (bind _returnvalue (Actor|GetActorOfClass "/Game/05_BluePrints/Spline/BP_SplinePath.BP_SplinePath_C"))
      (Variables|Default|SetSplineRef _returnvalue)
      (bind _returnvalue_2 (Actor|GetActorOfClass "/Game/05_BluePrints/Spline/BP_SplinePath1.BP_SplinePath1_C"))
      (Variables|Default|SetSpline2 _returnvalue_2)
      (bind _returnvalue_3 (Actor|GetActorOfClass "/Game/05_BluePrints/Spline/BP_SplinePath2.BP_SplinePath2_C"))
      (Variables|Default|SetSpline3 _returnvalue_3)
      (bind _returnvalue_4 (Actor|GetActorOfClass "/Game/05_BluePrints/Spline/BP_SplinePath3.BP_SplinePath3_C"))
      (Variables|Default|SetSpline4 _returnvalue_4)
      (bind _returnvalue_5 (Actor|GetActorOfClass "/Game/05_BluePrints/Spline/BP_SplinePath4.BP_SplinePath4_C"))
      (Variables|Default|SetSpline5 _returnvalue_5)
      (bind _returnvalue_6 (Actor|GetActorOfClass "/Game/05_BluePrints/Spline/BP_SplinePath5.BP_SplinePath5_C"))
      (Variables|Default|SetSpline6 _returnvalue_6))
    (:then_1
      (bind _asbp_ardu_pawn (Utilities|Casting|CastToBP_ArduPawn (Game|Player|GetPlayerPawn 0)))
      (Variables|Default|SetAs%20BP%20Ardu%20Pawn _asbp_ardu_pawn)
      (EventDispatchers|BindEventtoMovimiento1 _asbp_ardu_pawn (delegate Custom|Move))
      (EventDispatchers|BindEventtoMovimiento2 _asbp_ardu_pawn (delegate Custom|Move2))
      (EventDispatchers|BindEventtoMovimiento3 _asbp_ardu_pawn (delegate Custom|Mov3))
      (EventDispatchers|BindEventtoMovimiento4 _asbp_ardu_pawn (delegate Custom|Mov4))
      (EventDispatchers|BindEventtoMovimiento5 _asbp_ardu_pawn (delegate Custom|Mov5))
      (EventDispatchers|BindEventtoMovimiento6 _asbp_ardu_pawn (delegate Custom|Mov6)))))

(fn ConstructionScript)